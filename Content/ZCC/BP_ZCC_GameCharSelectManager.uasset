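; BP_ZCC_GameCharSelectManager is an actor that keeps a character creator in sync with the game's currently selected character.
; On BeginPlay it binds to the current-character change event of BP_ZCC_GameExample_Mgr, obtained through the ZCC game subsystem, then spawns a BP_ZCC_CreatorManager at its own transform.
; It immediately re-broadcasts the current character to initialize the view.
; Each change passes that character's Creation data to the spawned creator manager.
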(event Custom|OnCurrentCharacterCreationChange
  (params (CharacterCreation :type ZCC%20Character%20Creation%20Structure))
  (bind _creatormanager (Variables|Default|GetCreatorManager))
  (Utilities|IsValid _creatormanager
    (:Is%20Valid
      (Default|SetCurrentCharacterCreation _creatormanager CharacterCreation))))

(event EventBeginPlay
  (bind _gamemanager (CallFunction|GetGameManager))
  (EventDispatchers|BindEventtoOnCurrentCharacterChange _gamemanager (EventDispatchers|CreateEvent :!event OnCurrentCharacterChange))
  (CallFunction|CreateCreator)
  (Default|CallOnCurrentCharacterChange _gamemanager (Variables|/Game/ZCC/BP_ZCC_GameExample_Mgr.BP_ZCC_GameExample_Mgr_C|GetCurrentCharacter _gamemanager)))

(event Collision|EventActorBeginOverlap
  (params (OtherActor :type Actor%20Object%20Reference)))

(event EventTick
  (params (DeltaSeconds :type Float%20%28single-precision%29)))

(fn ConstructionScript)

(fn GetGameManager
  (return (Class|ZCCGameSubsystem|GetManagerbyClass (Subsystems|GetZCCGameSubsystem) "/Game/ZCC/BP_ZCC_GameExample_Mgr.BP_ZCC_GameExample_Mgr_C")))

(fn OnCurrentCharacterChange
  (params (Character :type F%20Struct%20ZCC%20Character%20Example%20Structure))
  (CallFunction|OnCurrentCharacterCreationChange (.Creation (Utilities|Struct|BreakFStruct_ZCC_Character_Example Character))))

(fn CreateCreator
  (bind _returnvalue (Game|SpawnActorfromClass "/Game/ZCC/Creator/BP_ZCC_CreatorManager.BP_ZCC_CreatorManager_C" (Transformation|GetActorTransform) "Undefined" "OverrideRootScale" 0 0 0))
  (Variables|Default|SetCreatorManager _returnvalue))