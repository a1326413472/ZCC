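; Manager actor for the ZCC character creator that owns the character currently being created.
; On BeginPlay it spawns an empty character from a default class and transform and stores it as the current character.
; SetCurrentCharacterCreation passes creation data to that character's ZCCCreationComponent through LoadCreation, provided the component is valid.
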(event EventBeginPlay
  (CallFunction|SpawnEmptyCharacter))

(event Collision|EventActorBeginOverlap
  (params (OtherActor :type Actor%20Object%20Reference)))

(event EventTick
  (params (DeltaSeconds :type Float%20%28single-precision%29)))

(fn ConstructionScript)

(fn SetCurrentCharacterCreation
  (params (InCharacterCreation :type ZCC%20Character%20Creation%20Structure))
  (bind _character (Variables|Default|GetCharacter))
  (bind _returnvalue (Actor|GetComponentbyClass _character "/Script/ACC.ZCCCreationComponent"))
  (Utilities|IsValid _returnvalue
    (:Is%20Valid
      (Class|ZCCCreationComponent|LoadCreation _returnvalue InCharacterCreation))))

(fn SpawnEmptyCharacter
  (bind _returnvalue (Game|SpawnActorfromClass (Variables|Config|GetDefaultCharacterClass) (Variables|Config|GetDefaultSpawnTransform) "Undefined" "MultiplyWithRoot" 0 0))
  (CallFunction|SetCurrentCharacter _returnvalue))

(fn SetCurrentCharacter
  (params (Character :type Actor%20Object%20Reference))
  (Variables|Default|SetCharacter Character))