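; BP_ZCC_GameExample_Mgr is the example game manager for ZCC, holding the save game and current character.
; StartLoadSaveGame waits briefly, then builds a fresh in-memory save rather than loading one from disk.
; That save is seeded with the "ZCC_HMN" species' default creation from ZCCCommonDAO.
; The first character is then selected through a validated index lookup and broadcast via OnCurrentCharacterChange.
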(event Custom|StartLoadSaveGame
  (Utilities|FlowControl|Delay 0.2)
  (CallFunction|CreateDefaultSaveGame)
  (CallFunction|SetupDefaultLoadedData))

(fn CreateDefaultSaveGame
  (bind _returnvalue (SaveGame|CreateSaveGameObject "/Game/ZCC/SaveGame/BP_ZCC_SaveGame_Example.BP_ZCC_SaveGame_Example_C"))
  (Variables|Default|SetCurrentSaveGame _returnvalue)
  (bind _speciedata (Class|ZCCCommonDAO|GetSpecieData (Class|ZCCGameplayStatics|GetDAObyClass "/Script/ACC.ZCCCommonDAO") "ZCC_HMN")
    (:True
      (bind _charactercreation (Class|ZCCSpecieDataAsset|GetDefaultCreation _speciedata)
        (:True
          (Utilities|Array|Add (Variables|/Game/ZCC/SaveGame/BP_ZCC_SaveGame_Example.BP_ZCC_SaveGame_Example_C|GetCharacters (Variables|Default|GetCurrentSaveGame)) (Utilities|Struct|MakeFStruct_ZCC_Character_Example "UnrealUnity" _charactercreation 15 999)))))))

(fn SetupDefaultLoadedData
  (CallFunction|SetCurrentCharacterfromIndex))

(fn SetCurrentCharacterfromIndex
  (params (Index :type Integer))
  (bind _output_get (Variables|Default|SetCurrentCharacterIndex Index))
  (if (.Valid (Get|GetCharacteratIndex _output_get))
    (CallFunction|SetCurrentCharacter (.Character (Get|GetCharacteratIndex _output_get)))))

(fn GetCharacteratIndex
  (params (Index :type Integer))
  (bind _currentsavegame (Variables|Default|GetCurrentSaveGame))
  (bind _characters (Variables|/Game/ZCC/SaveGame/BP_ZCC_SaveGame_Example.BP_ZCC_SaveGame_Example_C|GetCharacters _currentsavegame))
  (Utilities|FlowControl|Sequence
    (:then_0
      (Utilities|IsValid _currentsavegame
        (:Is%20Valid
          (if (Utilities|Array|IsValidIndex _characters Index)
            (return (Utilities|Array|Get(acopy) _characters Index) true)))))
    (:then_1
      (return "" false))))

(fn SetCurrentCharacter
  (params (Character :type F%20Struct%20ZCC%20Character%20Example%20Structure))
  (bind _output_get (Variables|Default|SetCurrentCharacter Character))
  (Default|CallOnCurrentCharacterChange _output_get))